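; Player character Blueprint handling weapon attachment, death and a few test hotkeys.
; AttachEquipmenttoHand snaps CurrentWeapon to the hand socket and unhides it.
; A SkinnyMonster hit at zero health, or DestroyandBacktoMenu, flags death on BP_GameHud and destroys the actor; the menu-loading node is unwired.
; N emits AI noise with a sound, while L zeroes and P raises every BP_ActorLight's spotlight intensity.
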(event `self.ReceiveBeginPlay`)

(event `self.AttachEquipmentToHand`
  (bind _currentweapon (`self.CurrentWeapon`))
  (`self.K2_AttachToComponent` (`self.CurrentWeapon`) (`self.Mesh`) (`self.GetInventoryAttachPoint` "Hands") "SnapToTarget" "SnapToTarget" "SnapToTarget" true)
  (set `BaseWeapon.MyPawn` self _currentweapon)
  (`SceneComponent.SetHiddenInGame` (`BaseWeapon.WeaponMesh` _currentweapon) false false)
  (`KismetSystemLibrary.PrintString` "Weapon Spawned"))

(event `self.ReceiveDestroyed`)

(event `Key|N`
  (params (Key :type "Key Structure" :default "AnyKey"))
  (bind _returnvalue (`self.K2_GetActorLocation`))
  (:`Pressed`
    (`PawnNoiseEmitterComponent.MakeNoise` (`self.PawnNoiseEmitterComp`) self 1.0 _returnvalue)
    (`GameplayStatics.PlaySoundAtLocation` "/Engine/EditorSounds/GamePreview/EndPlayInEditor_Cue.EndPlayInEditor_Cue" _returnvalue)))

(event `self.CapsuleComponent.OnComponentHit`
  (params (HitComponent :type "PrimitiveComponent Object Reference") (OtherActor :type "Actor Object Reference") (OtherComp :type "PrimitiveComponent Object Reference") (NormalImpulse :type "Vector Structure") (Hit :type "HitResult Structure (by ref)"))
  (cast `SkinnyMonster` OtherActor)
  (if (<= (`self.CurrentHealth`) 0.0)
    (set `self.CurrentHealth` 0.0 :!label _label)
    (`KismetSystemLibrary.PrintString` "Dead")
    (bind _outactors (`GameplayStatics.GetAllActorsOfClass` "/Game/BluePrints/Core/BP_GameHud.BP_GameHud_C"))
    (set `/Game/BluePrints/Core/BP_GameHud.IsCharacterDead` true (`KismetArrayLibrary.Array_Get` _outactors))
    (`self.K2_DestroyActor`)))

(event `self.DestroyAndBackToMenu`
  (goto _label))

(event `Key|L`
  (params (Key :type "Key Structure" :default "AnyKey"))
  (:`Pressed`
    (bind _outactors (`GameplayStatics.GetAllActorsOfClass` "/Game/BluePrints/Items/Assets/BP_ActorLight.BP_ActorLight_C"))
    (for _array_element _outactors
      (`LightComponent.SetIntensity` (`Actor_Light.SpotLightComp` _array_element) 0.0))))

(event `Key|P`
  (params (Key :type "Key Structure" :default "AnyKey"))
  (:`Pressed`
    (bind _outactors (`GameplayStatics.GetAllActorsOfClass` "/Game/BluePrints/Items/Assets/BP_ActorLight.BP_ActorLight_C"))
    (for _array_element _outactors
      (bind _spotlightcomp (`Actor_Light.SpotLightComp` _array_element))
      (`LightComponent.SetIntensity` _spotlightcomp (+ (`LightComponentBase.Intensity` _spotlightcomp) 100.0)))))

(fn `UserConstructionScript`)