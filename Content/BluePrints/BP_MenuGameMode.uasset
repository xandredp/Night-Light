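; BP_MenuGameMode is the menu game mode that manages mouse, input mode and background audio around level start.
; On BeginPlay it shows the BP_PlayController cursor, switches to game-and-UI input and plays a timeline that drives the AudioBg volume multiplier.
; OnLevelStart hides the cursor, sets game-only input and reverses the same timeline to run the volume change backwards.
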(event `self.ReceiveBeginPlay`
  (bind _asbp_play_controller (cast `/Game/BluePrints/Core/BP_PlayController` (`GameplayStatics.GetPlayerController` 0)))
  (set `PlayerController.bShowMouseCursor` true _asbp_play_controller)
  (`WidgetBlueprintLibrary.SetInputMode_GameAndUIEx` _asbp_play_controller)
  (bind (_direction _vol_audio) (`Timeline|Timeline_BG VolumeAdjustifer` :!label _label)
    (:`Update`
      (`AudioComponent.SetVolumeMultiplier` (`self.Audio_bg`) _vol_audio))))

(event `OnLevelStart`
  (bind _asbp_play_controller (cast `/Game/BluePrints/Core/BP_PlayController` (`GameplayStatics.GetPlayerController` 0)))
  (set `PlayerController.bShowMouseCursor` false _asbp_play_controller)
  (`WidgetBlueprintLibrary.SetInputMode_GameOnly` _asbp_play_controller)
  (goto _label :!via `Reverse`))

(fn `UserConstructionScript`)