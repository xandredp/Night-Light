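; An actor component that plays footstep sounds for an owning BP_NBCharacter.
; Each tick, while the character moves on the ground farther than Stride from the last footstep location, it line-traces downward.
; If the hit physical material is Floor_PhysMat, it plays a dry footstep cue at the impact and stores that point as the last footstep location.
; Other surfaces play no sound and leave the stored location unchanged.
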(event `self.ReceiveTick`
  (params (DeltaSeconds :type "Float (single-precision)"))
  (bind _character (`self.Character`))
  (bind _returnvalue (`Actor.K2_GetActorLocation` _character))
  (bind _asbp_nbcharacter (cast `/Game/BluePrints/Character/BP_NBCharacter` (`self.GetOwner`)))
  (bind _output_get (set `self.Character` _asbp_nbcharacter))
  (if (and (> (`KismetMathLibrary.VSize` (- (`Actor.K2_GetActorLocation` (`self.Character`)) (`self.Last Footstep Location`))) (`self.Stride`)) (`NavMovementComponent.IsMovingOnGround` (`Pawn.GetMovementComponent` _output_get)))
    (bind (_outhit _returnvalue_2) (`KismetSystemLibrary.LineTraceSingle` _returnvalue (- _returnvalue (`KismetMathLibrary.MakeVector` 0.0 0.0 (* (`CapsuleComponent.CapsuleHalfHeight` (`Character.CapsuleComponent` _character)) 2.0))) "TraceTypeQuery1"))
    (bind (_bblockinghit _binitialoverlap _time _location _impactpoint _normal _impactnormal _physmat) (`GameplayStatics.BreakHitResult` _outhit))
    (if (and _returnvalue_2 (== _physmat "/Game/Meshes/Floor/Floor_PhysMat.Floor_PhysMat"))
      (`GameplayStatics.PlaySoundAtLocation` "/Game/Sound/SFX/Footsteps/Footstep_Dry_Cue.Footstep_Dry_Cue" _location)
      (set `self.Last Footstep Location` _location))))