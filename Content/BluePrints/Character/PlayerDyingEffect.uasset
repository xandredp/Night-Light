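; Player death effect Blueprint that applies post-process settings and sends a physics sphere tumbling when play begins.
; On BeginPlay it copies PPSettings into its PostProcess component and hits the Sphere with a random-direction impulse at a random location vector.
; A coin flip then fires either the LeftForce or RightForce impulse, so the motion varies each time.
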(event `self.ReceiveBeginPlay`
  (bind _returnvalue (* (`KismetMathLibrary.RandomUnitVector`) 650.0))
  (set `PostProcessComponent.Settings` (`self.PPSettings`) (`self.PostProcess`))
  (`PrimitiveComponent.AddImpulseAtLocation` (`self.Sphere`) _returnvalue _returnvalue "None")
  (if (`KismetMathLibrary.RandomBool`)
    (`RadialForceComponent.FireImpulse` (`self.leftForce`))
    (else
      (`RadialForceComponent.FireImpulse` (`self.RightForce`)))))

(fn `UserConstructionScript`)