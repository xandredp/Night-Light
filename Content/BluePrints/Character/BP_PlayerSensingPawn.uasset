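; BP_PlayerSensingPawn is a cone-shaped sensor that tells the player character's current torch which skinny AI enemies are in range.
; Cone overlaps add each NBSkinnyAI to the torch's EnemyPawns and set it as EnemyPawn.
; Leaving the cone removes it from the list and resets EnemyPawn to a stored variable.
; An electricity-arc beam effect remains in the graph but never runs, as SpawnParticleEffect is empty.
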(event `self.SpawnParticleEffect`
  (params (Pawn :type "Pawn Object Reference")))

(event `self.Cone.OnComponentBeginOverlap`
  (params (OverlappedComponent :type "PrimitiveComponent Object Reference") (OtherActor :type "Actor Object Reference") (OtherComp :type "PrimitiveComponent Object Reference") (OtherBodyIndex :type Integer) (bFromSweep :type Boolean) (SweepResult :type "HitResult Structure (by ref)"))
  (bind _currenttorch (`NBCharacter.CurrentTorch` (`self.NBCharacter`)))
  (bind _asnbskinny_ai (cast `NBSkinnyAI` OtherActor))
  (`/Engine/EditorBlueprintResources/StandardMacros.IsValid` _currenttorch
    (:`Is Valid`
      (set `BaseTorch.EnemyPawn` _asnbskinny_ai _currenttorch)
      (`KismetArrayLibrary.Array_Add` (`BaseTorch.EnemyPawns` _currenttorch) _asnbskinny_ai))))

(event `self.Cone.OnComponentEndOverlap`
  (params (OverlappedComponent :type "PrimitiveComponent Object Reference") (OtherActor :type "Actor Object Reference") (OtherComp :type "PrimitiveComponent Object Reference") (OtherBodyIndex :type Integer))
  (bind _currenttorch (`NBCharacter.CurrentTorch` (`self.NBCharacter`)))
  (bind _asnbskinny_ai (cast `NBSkinnyAI` OtherActor))
  (`/Engine/EditorBlueprintResources/StandardMacros.IsValid` _currenttorch
    (:`Is Valid`
      (set `BaseTorch.EnemyPawn` (`self.NewVar_0`) _currenttorch)
      (`KismetArrayLibrary.Array_RemoveItem` (`BaseTorch.EnemyPawns` _currenttorch) _asnbskinny_ai))))

(fn `UserConstructionScript`)