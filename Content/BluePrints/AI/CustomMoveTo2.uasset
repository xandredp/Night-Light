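; CustomMoveTo2 is a behavior tree task that issues an AI move for the pawn controlled by BP_NBAIController.
; Its work runs on Tick rather than on Execute, which is empty, and targets the pawn's own current location.
; Both success and failure finish the task as successful, while a failed controller cast leaves it unfinished.
; A player-location lookup is present but unused.
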(event `self.ReceiveTick`
  (params (OwnerActor :type "Actor Object Reference") (DeltaSeconds :type "Float (single-precision)"))
  (bind _asbp_nbaicontroller (cast `/Game/BluePrints/Enemies/BP_NBAIController` (`AIBlueprintHelperLibrary.GetAIController` OwnerActor)))
  (bind _returnvalue (`Controller.K2_GetPawn` _asbp_nbaicontroller))
  (`|AIMoveTo` _returnvalue (`Actor.K2_GetActorLocation` _returnvalue) null 5.0 true
    (:`OnSuccess`
      (`KismetSystemLibrary.PrintString` "FinishExecute - normal" false false)
      (`self.FinishExecute` true))
    (:`OnFail`
      (`KismetSystemLibrary.PrintString` "FinishExecute Failed" false false)
      (`self.FinishExecute` true))))

(event `self.ReceiveExecute`
  (params (OwnerActor :type "Actor Object Reference")))