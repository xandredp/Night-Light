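; Game HUD Blueprint that shows the in-game UI and handles the switch to the end screen on character death.
; BeginPlay resets IsCharacterDead, adds WB_Ingame to the viewport and enables input for the owning player controller.
; Tick polls that flag; while set, it adds a new WB_Endscene every frame and clears the HUDIngame reference without removing that widget.
; A two-second delay then opens the MainMenu level.
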(event `self.ReceiveTick`
  (params (DeltaSeconds :type "Float (single-precision)"))
  ;[1 1 1] Setup Widgets
  (if (`self.IsCharacterDead`)
    (bind _returnvalue (`|CreateWidget` "/Game/UI/WB_Endscene.WB_Endscene_C"))
    (set `self.HUDIngame` null)
    (`UserWidget.AddToViewport` _returnvalue 0)
    (`KismetSystemLibrary.Delay` 2.0)
    (`GameplayStatics.OpenLevel` "MainMenu")))

(event `self.ReceiveBeginPlay`
  ;[1 1 1] Setup Widgets
  (`|ExecutionSequence`
    (:`then_0`
      (set `self.IsCharacterDead` false)
      (bind _returnvalue (`|CreateWidget` "/Game/UI/WB_Ingame.WB_Ingame_C"))
      (bind _output_get (set `self.HUDIngame` _returnvalue))
      (`UserWidget.AddToViewport` _output_get 0))
    (:`then_5`
      (`self.EnableInput` (`self.GetOwningPlayerController`)))))

(fn `UserConstructionScript`)