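; BP_PlayGameMode is a game mode Blueprint that switches audio to follow the General, Alert, Combat or Death state.
; CheckSound compares GameModeState with CurrentGameMode, sets and plays the Audio component's sound on a change, then records the new state.
; An unmatched state loops back through the same checks.
; BeginPlay and Tick are empty, and the looping timer meant to call CheckSound is disconnected.
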(event `self.ReceiveBeginPlay`)

(event `CheckSound`
  (bind _audio (`self.Audio`))
  (bind _audio_2 (`self.Audio`))
  (bind _audio_3 (`self.Audio`))
  (bind _audio_4 (`self.Audio`))
  (if (not (`|EnumEquality` (`self.GameModeState`) (`self.CurrentGameMode`)))
    (if (`|EnumEquality` (`self.GameModeState`) "General") :!label _label
      (`AudioComponent.SetSound` _audio_2 null)
      (`AudioComponent.Play` _audio_2 0.0)
      (set `self.CurrentGameMode` "General")
      (elif (`|EnumEquality` (`self.GameModeState`) "Alert")
        (`AudioComponent.SetSound` _audio_3 null)
        (`AudioComponent.Play` _audio_3 0.0)
        (set `self.CurrentGameMode` "Alert")
        (elif (`|EnumEquality` (`self.GameModeState`) "Combat")
          (`AudioComponent.SetSound` _audio_4 null)
          (`AudioComponent.Play` _audio_4 0.0)
          (set `self.CurrentGameMode` "Combat")
          (elif (`|EnumEquality` (`self.GameModeState`) "Death")
            (`AudioComponent.SetSound` _audio null)
            (`AudioComponent.Play` _audio 0.0)
            (set `self.CurrentGameMode` "Death")
            (else
              (goto _label))))))))

(event `self.ReceiveTick`
  (params (DeltaSeconds :type "Float (single-precision)")))

(fn `UserConstructionScript`)