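; Wave spawner that defines five monster waves, each spawned at randomly picked points from that wave's spawn list.
; BeginPlay resets WaveIndex, then runs one Sequence that checks each wave once, with no timer or re-trigger.
; Each wave requires zero Skinny and Tanky monsters; later waves also require a matching WaveIndex, which increments inside spawn loops.
; Waves 3 to 5 spawn two monster classes using per-type counts.
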(event `self.ReceiveBeginPlay`
  (bind (_whattospawn _numbertospawn _wheretospawn) (break `/Game/BluePrints/Spawning/Wave1` (`self.Wave1`)))
  (bind (_whattospawn_2 _numbertospawn_2 _wheretospawn_2) (break `/Game/BluePrints/Spawning/Wave2` (`self.Wave2`)))
  (bind (_whattospawn_3 _numbertospawn_3 _wheretospawn_3) (break `/Game/BluePrints/Spawning/Wave3` (`self.Wave3`)))
  (bind (_whattospawn_4 _numbertospawn_4 _wheretospawn_4) (break `/Game/BluePrints/Spawning/Wave4` (`self.Wave4`)))
  (bind (_whattospawn_5 _numbertospawn_5 _wheretospawn_5) (break `/Game/BluePrints/Spawning/Wave5` (`self.Wave5`)))
  ;[1 1 1] Reset Wave index
  (if (not (== (`self.WaveIndex`) 1))
    (set `self.WaveIndex` 1))
  (`|ExecutionSequence`
    (:`then_0`
      ;[1 1 1] Spawning 1st Wave
      (bind _iswaveready (`self.Is Wave Ready`))
      (if _iswaveready
        (for _ (range (+ _numbertospawn 1))
          (bind _random_spawn_point_index (`self.Get Random Spawn Point` _wheretospawn))
          (`|SpawnActorFromClass` _whattospawn (`self.GetTransform` (`KismetArrayLibrary.Array_Get` _wheretospawn _random_spawn_point_index)) "AdjustIfPossibleButAlwaysSpawn" "OverrideRootScale")
          ;[1 1 1] Increment Wave index to get ready to spawn Wave 2
          (bind _result (`/Engine/EditorBlueprintResources/StandardMacros.IncrementInt` (`self.WaveIndex`))
            (:`  `
              (set `self.WaveIndex` _result))))))
    (:`then_1`
      ;[1 1 1] Is the wave ready and is the current wave 2?
      (bind _iswaveready_2 (`self.Is Wave Ready`))
      (if _iswaveready_2
        (if (== (`self.WaveIndex`) 2)
          ;[1 1 1] Spawning 2nd wave
          (for _ (range (+ _numbertospawn_2 1))
            (bind _random_spawn_point_index_2 (`self.Get Random Spawn Point` _wheretospawn_2))
            (`|SpawnActorFromClass` _whattospawn_2 (`self.GetTransform` (`KismetArrayLibrary.Array_Get` _wheretospawn_2 _random_spawn_point_index_2)) "AdjustIfPossibleButAlwaysSpawn" "OverrideRootScale")
            ;[1 1 1] Increment Wave index to get ready to spawn Wave 3
            (bind _result_2 (`/Engine/EditorBlueprintResources/StandardMacros.IncrementInt` (`self.WaveIndex`))
              (:`  `
                (set `self.WaveIndex` _result_2)))))))
    (:`then_2`
      ;[1 1 1] is the wave ready and is the current wave 3?
      (bind _iswaveready_3 (`self.Is Wave Ready`))
      (if _iswaveready_3
        (if (== (`self.WaveIndex`) 3)
          ;[1 1 1] Spawning 3rd wave
          (bind (_index_0 _index_1) (`self.Get Number To Spawn` _numbertospawn_3))
          (`|ExecutionSequence`
            (:`then_0`
              (for _ (`|MakeArray` _index_0)
                (bind _random_spawn_point_index_3 (`self.Get Random Spawn Point` _wheretospawn_3))
                (`|SpawnActorFromClass` (`KismetArrayLibrary.Array_Get` _whattospawn_3) (`self.GetTransform` (`KismetArrayLibrary.Array_Get` _wheretospawn_3 _random_spawn_point_index_3)) "Undefined" "OverrideRootScale")))
            (:`then_1`
              (for _ (`|MakeArray` _index_1)
                (bind _random_spawn_point_index_4 (`self.Get Random Spawn Point` _wheretospawn_3))
                (`|SpawnActorFromClass` (`KismetArrayLibrary.Array_Get` _whattospawn_3 1) (`self.GetTransform` (`KismetArrayLibrary.Array_Get` _wheretospawn_3 _random_spawn_point_index_4)) "Undefined" "OverrideRootScale")
                ;[1 1 1] Increment Wave index to get ready to spawn Wave 4
                (bind _result_3 (`/Engine/EditorBlueprintResources/StandardMacros.IncrementInt` (`self.WaveIndex`))
                  (:`  `
                    (set `self.WaveIndex` _result_3)))))))))
    (:`then_3`
      ;[1 1 1] Is the current wave 4?
      (bind _iswaveready_4 (`self.Is Wave Ready`))
      (if _iswaveready_4
        (if (== (`self.WaveIndex`) 4)
          ;[1 1 1] Spawning 4th wave
          (bind (_index_0_2 _index_1_2) (`self.Get Number To Spawn` _numbertospawn_4))
          (`|ExecutionSequence`
            (:`then_0`
              (for _ (`|MakeArray` _index_0_2)
                (bind _random_spawn_point_index_5 (`self.Get Random Spawn Point` _wheretospawn_4))
                (`|SpawnActorFromClass` (`KismetArrayLibrary.Array_Get` _whattospawn_4) (`self.GetTransform` (`KismetArrayLibrary.Array_Get` _wheretospawn_4 _random_spawn_point_index_5)) "AdjustIfPossibleButAlwaysSpawn" "OverrideRootScale")))
            (:`then_1`
              (for _ (`|MakeArray` _index_1_2)
                (bind _random_spawn_point_index_6 (`self.Get Random Spawn Point` _wheretospawn_4))
                (`|SpawnActorFromClass` (`KismetArrayLibrary.Array_Get` _whattospawn_4 1) (`self.GetTransform` (`KismetArrayLibrary.Array_Get` _wheretospawn_4 _random_spawn_point_index_6)) "AdjustIfPossibleButAlwaysSpawn" "OverrideRootScale")
                ;[1 1 1] Increment Wave index to get ready to spawn Wave 5
                (bind _result_4 (`/Engine/EditorBlueprintResources/StandardMacros.IncrementInt` (`self.WaveIndex`))
                  (:`  `
                    (set `self.WaveIndex` _result_4)))))))))
    (:`then_4`
      ;[1 1 1] Is the wave ready and is current wave 5?
      (bind _iswaveready_5 (`self.Is Wave Ready`))
      (if _iswaveready_5
        (if (== (`self.WaveIndex`) 5)
          ;[1 1 1] Spawning 5th wave
          (bind (_index_0_3 _index_1_3) (`self.Get Number To Spawn` _numbertospawn_5))
          (`|ExecutionSequence`
            (:`then_0`
              (for _ (`|MakeArray` _index_0_3)
                (bind _random_spawn_point_index_7 (`self.Get Random Spawn Point` _wheretospawn_5))
                (`|SpawnActorFromClass` (`KismetArrayLibrary.Array_Get` _whattospawn_5) (`self.GetTransform` (`KismetArrayLibrary.Array_Get` _wheretospawn_5 _random_spawn_point_index_7)) "AdjustIfPossibleButAlwaysSpawn" "OverrideRootScale")))
            (:`then_1`
              (for _ (`|MakeArray` _index_1_3)
                (bind _random_spawn_point_index_8 (`self.Get Random Spawn Point` _wheretospawn_5))
                (`|SpawnActorFromClass` (`KismetArrayLibrary.Array_Get` _whattospawn_5 1) (`self.GetTransform` (`KismetArrayLibrary.Array_Get` _wheretospawn_5 _random_spawn_point_index_8)) "AdjustIfPossibleButAlwaysSpawn" "OverrideRootScale")))))))))

(fn `Get Number To Spawn`
  (params (`Number To Spawn Array` :type "Array of Integer"))
  (returns (`Index 0` :type Integer) (`Index 1` :type Integer))
  (locals (Index0Ammount :type Integer) (Index1Ammount :type Integer))
  (bind _output_get (set `local.Index0Ammount` (`KismetArrayLibrary.Array_Get` `Number To Spawn Array`)))
  (bind _output_get_2 (set `local.Index1Ammount` (`KismetArrayLibrary.Array_Get` `Number To Spawn Array` 1)))
  (return _output_get _output_get_2))

(fn `Get Random Spawn Point`
  (params (SpawnPoints :type "Array of Actor Object Reference"))
  (returns (`Random Spawn Point Index` :type Integer))
  (locals (`Spawn Points Array Length` :type Integer))
  (bind _output_get (set `local.Spawn Points Array Length` (`KismetArrayLibrary.Array_Length` SpawnPoints)))
  (bind _output_get_2 (set `self.RandomWhereToSpawnIndex` (`KismetMathLibrary.RandomIntegerInRange` 0 _output_get)))
  (return _output_get_2))

(fn `Is Wave Ready`
  (returns (IsWaveReady :type Boolean))
  (locals (SkinnyMonsterAmmount :type Integer) (TankyMonsterAmmount :type Integer))
  (bind _outactors (`GameplayStatics.GetAllActorsOfClass` "/Game/BluePrints/Enemies/BP_SkinnyMonster.BP_SkinnyMonster_C"))
  (bind _output_get (set `local.SkinnyMonsterAmmount` (`KismetArrayLibrary.Array_Length` _outactors)))
  (bind _outactors_2 (`GameplayStatics.GetAllActorsOfClass` "/Game/BluePrints/Enemies/BP_TankyMonster.BP_TankyMonster_C"))
  (bind _output_get_2 (set `local.TankyMonsterAmmount` (`KismetArrayLibrary.Array_Length` _outactors_2)))
  (return (and (== _output_get_2 0) (== _output_get 0))))

(fn `UserConstructionScript`)