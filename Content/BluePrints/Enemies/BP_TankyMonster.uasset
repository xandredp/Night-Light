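; BP_TankyMonster is an enemy that charges at the player and switches to a charge attack on contact.
; A looping timer traces forward from an arrow; on a player hit off cooldown, it passes the charge target to its AI controller and raises walk speed.
; Anim Blueprint flags drive charging, switching to attack when the player overlaps a trigger sphere.
; A separate DecreaseCharacterHealth event applies attack damage to the player.
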(event `self.ReceiveBeginPlay`
  (bind _returnvalue (`AIBlueprintHelperLibrary.GetAIController` self))
  (bind _asbp_my_my_aicontroller (cast `/Game/BluePrints/Enemies/BP_MyMyAIController` _returnvalue))
  (set `self.TankyAIController` _asbp_my_my_aicontroller)
  (bind _astanky_anim_bp (cast `/Game/BluePrints/Animations/TankyMonster/TankyAnimBP` (`SkeletalMeshComponent.GetAnimInstance` (`self.Mesh`))))
  (set `self.TankyMonsterAnimBP` _astanky_anim_bp)
  (`KismetSystemLibrary.K2_SetTimerDelegate` (delegate `self.LineTrace`) (`self.ChargingCooldown`) true))

(event `self.ReceiveTick`
  (params (DeltaSeconds :type "Float (single-precision)")))

(event `self.LineTrace`
  (bind _arrow1 (`self.Arrow1`))
  (bind _returnvalue (`SceneComponent.K2_GetComponentLocation` _arrow1))
  (bind _outhit (`KismetSystemLibrary.LineTraceSingle` :`Start` _returnvalue :`End` (+ _returnvalue (* (`SceneComponent.GetForwardVector` _arrow1) 1000.0)) :`TraceChannel` "TraceTypeQuery3" :`DrawDebugType` "ForDuration"))
  (bind _asbp_nbcharacter (cast `/Game/BluePrints/Character/BP_NBCharacter` (`.HitActor` (`GameplayStatics.BreakHitResult` _outhit)))
    (:`then`
      (set `self.PlayerCharacter` _asbp_nbcharacter)
      (if (>= (- (`GameplayStatics.GetTimeSeconds`) (`self.LastChargingTime`)) (`self.ChargingCooldown`))
        (`MyAIController.SetLocationToCharge` (`self.TankyAIController`) (`SceneComponent.K2_GetComponentLocation` (`/Game/BluePrints/Character/BP_NBCharacter.Charging Point` (`self.PlayerCharacter`))))
        (`MyAIController.SetChargeTarget` (`self.TankyAIController`) (`self.PlayerCharacter`))
        (set `CharacterMovementComponent.MaxWalkSpeed` (`self.ChargingSpeed`) (`self.TankyMoveComp`))
        (set `self.LastChargingTime` (`GameplayStatics.GetTimeSeconds`))
        (set `SkinnyMonsterAnimInstance.CanCharge` true (`self.TankyMonsterAnimBP`))
        (`KismetSystemLibrary.Delay` 2.0)))
    (:`CastFailed`
      (`MyAIController.ResetChargeTarget` (`self.TankyAIController`)))))

(event `self.DecreaseCharacterHealth`
  (bind _asbp_nbcharacter (cast `/Game/BluePrints/Character/BP_NBCharacter` (`GameplayStatics.GetPlayerCharacter` 0)))
  (`NBCharacter.DecreaseHealth` _asbp_nbcharacter (`self.AttackDamage`)))

(event `self.AttackAnimTriggerSphere.OnComponentBeginOverlap`
  (params (OverlappedComponent :type "PrimitiveComponent Object Reference") (OtherActor :type "Actor Object Reference") (OtherComp :type "PrimitiveComponent Object Reference") (OtherBodyIndex :type Integer) (bFromSweep :type Boolean) (SweepResult :type "HitResult Structure (by ref)"))
  (cast `/Game/BluePrints/Character/BP_NBCharacter` OtherActor)
  (if (`SkinnyMonsterAnimInstance.CanCharge` (`self.TankyMonsterAnimBP`))
    (set `SkinnyMonsterAnimInstance.CanCharge` false (`self.TankyMonsterAnimBP`))
    (set `SkinnyMonsterAnimInstance.CanChargeAttack` true (`self.TankyMonsterAnimBP`))
    (`SceneComponent.SetHiddenInGame` (`self.AttackRangeSphere`) true false)))

(fn `UserConstructionScript`)