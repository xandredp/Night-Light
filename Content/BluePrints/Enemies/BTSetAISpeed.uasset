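; Behavior tree task that resets the tanky monster's walk speed to its usual value.
; On execute, it caches the owner's AI controller and the controlled BP_TankyMonster pawn.
; It then copies the monster's UsualSpeed into its movement component's MaxWalkSpeed and finishes successfully.
; If the pawn is not a tanky monster, the task stops without calling FinishExecute.
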(event `self.ReceiveExecute`
  (params (OwnerActor :type "Actor Object Reference"))
  (bind _tankymonster (`self.TankyMonster`))
  (bind _returnvalue (`AIBlueprintHelperLibrary.GetAIController` OwnerActor))
  (bind _asbp_my_my_aicontroller (cast `/Game/BluePrints/Enemies/BP_MyMyAIController` _returnvalue)
    (:`then`
      ;[1 1 1] Initialize
      (set `self.TankyMonsterAICtrl` _asbp_my_my_aicontroller))
    (:`CastFailed`
      _))
  (bind _asbp_tanky_monster (cast `/Game/BluePrints/Enemies/BP_TankyMonster` (`Controller.K2_GetPawn` _returnvalue)))
  (set `self.TankyMonster` _asbp_tanky_monster)
  (set `CharacterMovementComponent.MaxWalkSpeed` (`TankyMonster.UsualSpeed` _tankymonster) (`TankyMonster.TankyMoveComp` _tankymonster))
  (`self.FinishExecute` true))