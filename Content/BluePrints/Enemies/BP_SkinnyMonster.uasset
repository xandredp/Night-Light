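; Skinny monster enemy Blueprint that damages the player, drops loot and reacts to light.
; Its events set the game mode's state and apply AttackDamage to the player character.
; Light toggles the mesh's material and its blocking of a custom trace channel, ignored in darkness.
; Drop logic spawns an item at the mesh and moves an existing key's pickup mesh, passing world position as relative location.
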(event `self.SetPlayModeState`
  (params (ChangeSoundState :type "EGameModeSoundType Enum" :default "General"))
  (bind _asbp_play_game_mode (cast `/Game/BluePrints/BP_PlayGameMode` (`GameplayStatics.GetGameMode`)))
  (set `PlayGameMode.GameModeState` ChangeSoundState _asbp_play_game_mode))

(event `self.DecreaseCharacterHealth`
  (bind _asbp_nbcharacter (cast `/Game/BluePrints/Character/BP_NBCharacter` (`GameplayStatics.GetPlayerCharacter` 0)))
  (`NBCharacter.DecreaseHealth` _asbp_nbcharacter (`self.AttackDamage`)))

(event `self.SpawnDropItems`
  (`|ExecutionSequence`
    (:`then_0`
      (if (`KismetSystemLibrary.IsValidClass` (`self.DropItemOnDeath`))
        (`|SpawnActorFromClass` (`self.DropItemOnDeath`) (`KismetMathLibrary.Conv_VectorToTransform` (`SceneComponent.K2_GetComponentLocation` (`self.Mesh`))) "Undefined" "OverrideRootScale")))
    (:`then_1`
      (if (`KismetSystemLibrary.IsValid` (`self.DropKeyOnDeath`))
        (`SceneComponent.K2_SetRelativeLocation` (`BaseInteractable.PickupSkeletalMesh` (`self.DropKeyOnDeath`)) (`SceneComponent.K2_GetComponentLocation` (`self.Mesh`)) false false)
        (else
          (`KismetSystemLibrary.PrintString` "Hello"))))))

(event `self.MonsterInLight`
  (params (isInLight :type Boolean))
  (bind _mesh (`self.Mesh`))
  (bind _mesh_2 (`self.Mesh`))
  (if isInLight
    (`PrimitiveComponent.SetMaterial` _mesh 0 "/Game/Textures/Monster/Mon_M.Mon_M")
    (`PrimitiveComponent.SetCollisionResponseToChannel` _mesh "ECC_GameTraceChannel1" "ECR_Block")
    (else
      (`PrimitiveComponent.SetMaterial` _mesh_2 0 "/Game/Textures/Monster/Mon_M_Darkness.Mon_M_Darkness")
      (`PrimitiveComponent.SetCollisionResponseToChannel` _mesh_2 "ECC_GameTraceChannel1" "ECR_Ignore"))))

(fn `UserConstructionScript`)