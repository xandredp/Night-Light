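; Behavior tree task that sends an enemy's pawn toward the player or, for a fleeing skinny monster, to a flee point.
; On execute it resets tanky monster speed, calls the move logic and finishes successfully without waiting for arrival.
; Only skinny monsters get move orders: fleeing ones speed up toward the first FleePoint found, issued per actor tag.
; Reaching it clears the flee flags and slows them; otherwise they pursue the player.
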(event `self.ReceiveExecute`
  (params (OwnerActor :type "Actor Object Reference"))
  (bind _returnvalue (`AIBlueprintHelperLibrary.GetAIController` OwnerActor))
  (bind _asbp_tanky_monster (cast `/Game/BluePrints/Enemies/BP_TankyMonster` OwnerActor)
    (:`then`
      (set `CharacterMovementComponent.MaxWalkSpeed` (`TankyMonster.UsualSpeed` _asbp_tanky_monster) (`TankyMonster.TankyMoveComp` _asbp_tanky_monster))
      (`self.MoveAiToPlayerCharacter`)
      (`self.FinishExecute` true))
    (:`CastFailed`
      (`self.MoveAiToPlayerCharacter`)
      (`self.FinishExecute` true))))

(event `MoveAiToPlayerCharacter`
  (bind _returnvalue (`Controller.K2_GetPawn` (stale `self.ReceiveExecute` _returnvalue)))
  (bind _asbp_skinny_monster (cast `/Game/BluePrints/Enemies/BP_SkinnyMonster` _returnvalue))
  (if (`/Game/BluePrints/Enemies/BP_SkinnyMonster.Fleeing2` _asbp_skinny_monster)
    (if (`/Game/BluePrints/Enemies/BP_SkinnyMonster.InMidFlee` _asbp_skinny_monster)
      (bind _movementresult (`|AIMoveTo` _asbp_skinny_monster (0.0 0.0 0.0) (`self.SavedFleePoint`))
        (:`then`
          (switch `EPathFollowingResult` _movementresult
            (:`Success`
              _)
            (:`Aborted`
              _))
          (set `/Game/BluePrints/Enemies/BP_SkinnyMonster.Fleeing2` false _asbp_skinny_monster)
          (set `/Game/BluePrints/Enemies/BP_SkinnyMonster.InMidFlee` false _asbp_skinny_monster)
          (bind _charactermovement (`Character.CharacterMovement` _asbp_skinny_monster))
          (set `CharacterMovementComponent.MaxWalkSpeed` 40.0 _charactermovement)))
      (else
        (`KismetSystemLibrary.PrintString` "fleeing" false)
        (set `CharacterMovementComponent.MaxWalkSpeed` 1000.0 _charactermovement)
        (for _array_element (`Actor.Tags` _asbp_skinny_monster)
          (`KismetSystemLibrary.PrintString` (`KismetStringLibrary.Conv_NameToString` _array_element) false true (struct :`G` 0.66 :`B` 1.0 :`A` 1.0) 0.5)
          (bind _outactors (`GameplayStatics.GetAllActorsOfClass` "/Game/BluePrints/Enemies/FleePoint.FleePoint_C"))
          (set `/Game/BluePrints/Enemies/BP_SkinnyMonster.InMidFlee` true _asbp_skinny_monster)
          (bind _item (`KismetArrayLibrary.Array_Get` _outactors))
          (set `self.SavedFleePoint` _item)
          (bind _movementresult_2 (`|AIMoveTo` _returnvalue (0.0 0.0 0.0) _item)
            (:`then`
              (switch `EPathFollowingResult` _movementresult_2
                (:`Success`
                  (set `/Game/BluePrints/Enemies/BP_SkinnyMonster.Fleeing2` false _asbp_skinny_monster)
                  (set `/Game/BluePrints/Enemies/BP_SkinnyMonster.InMidFlee` false _asbp_skinny_monster)
                  (set `CharacterMovementComponent.MaxWalkSpeed` 40.0 _charactermovement))))))))
    (else
      (`|AIMoveTo` _returnvalue (0.0 0.0 0.0) (`GameplayStatics.GetPlayerCharacter` 0)))))

(fn `NewFunction_0`
  (params (TargetArray :type "Array of /Game/BluePrints/Enemies/FleePoint Object Reference (by ref)") (Index :type Integer))
  (returns (Item :type "/Game/BluePrints/Enemies/FleePoint Object Reference"))
  (return (`KismetArrayLibrary.Array_Get` TargetArray Index)))