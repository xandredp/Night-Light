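; Base torch weapon Blueprint that handles the visual and audio feedback of a stun activation.
; TorchActivatedEvent plays the stun sound and applies the stun intensity and radius to the spotlight, without resetting them here.
; If EnemyPawn is a BP_NBSkinnyAI, a UV laser beam emitter attaches to its mesh and targets the torch light.
; The beam is destroyed after a short delay, then current energy is printed for debugging.
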(event `self.TorchActivatedEvent`
  (bind _torchspotlight (`self.TorchSpotlight`))
  (bind _torchspotlight_2 (`self.TorchSpotlight`))
  (`GameplayStatics.PlaySoundAtLocation` _torchspotlight_2 (`self.StunActivationSound`) (`SceneComponent.K2_GetComponentLocation` _torchspotlight_2))
  (`LightComponent.SetIntensity` _torchspotlight (`self.StunIntensity`))
  (`PointLightComponent.SetAttenuationRadius` _torchspotlight (`self.StunAttenuationRadious`))
  (bind _asbp_nbskinny_ai (cast `/Game/BluePrints/Enemies/BP_NBSkinnyAI` (`self.EnemyPawn`)))
  (bind _returnvalue (`GameplayStatics.SpawnEmitterAttached` "/Game/Effects/P_UVLight_Laser.P_UVLight_Laser" (`Character.Mesh` _asbp_nbskinny_ai)))
  (`ParticleSystemComponent.SetBeamTargetPoint` _returnvalue 0 (`SceneComponent.K2_GetComponentLocation` (`self.TorchSpotlight`)) 0)
  (`KismetSystemLibrary.Delay` 2.0)
  (`ActorComponent.K2_DestroyComponent` _returnvalue)
  (`KismetSystemLibrary.PrintString` (`KismetStringLibrary.Conv_DoubleToString` (`self.CurrentEnergy`))))

(fn `UserConstructionScript`)