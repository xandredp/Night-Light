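; BP_CrackingObjForLight is an item actor that displays its energy level on a floating widget bar.
; BeginPlay caches the WB_EnergyBar widget and hides it, and InRangeSphere overlaps by any actor show or hide it.
; Each Tick sets the bar's fill from Energy over MaxEnergy and turns the widget toward the player camera on yaw only, keeping it upright.
; This Blueprint only reads Energy and never changes it.
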(event `self.ReceiveBeginPlay`
  (bind _aswb_energy_bar (cast `/Game/UI/WB_EnergyBar` (`WidgetComponent.GetUserWidgetObject` (`self.Widget`))))
  (set `self.EnergyBarWB` _aswb_energy_bar)
  (`SceneComponent.SetVisibility` (`self.Widget`) false false))

(event `self.ReceiveTick`
  (params (DeltaSeconds :type "Float (single-precision)"))
  (bind _widget (`self.Widget`))
  (`self.UpdateEnergyBar`)
  (`SceneComponent.K2_SetWorldRotation` _widget (`KismetMathLibrary.MakeRotator` 0.0 0.0 (.yaw (`KismetMathLibrary.FindLookAtRotation` (`SceneComponent.K2_GetComponentLocation` _widget) (`PlayerCameraManager.GetCameraLocation` (`GameplayStatics.GetPlayerCameraManager` 0))))) false false))

(event `self.InRangeSphere.OnComponentBeginOverlap`
  (params (OverlappedComponent :type "PrimitiveComponent Object Reference") (OtherActor :type "Actor Object Reference") (OtherComp :type "PrimitiveComponent Object Reference") (OtherBodyIndex :type Integer) (bFromSweep :type Boolean) (SweepResult :type "HitResult Structure (by ref)"))
  (`SceneComponent.SetVisibility` (`self.Widget`) true false))

(event `self.InRangeSphere.OnComponentEndOverlap`
  (params (OverlappedComponent :type "PrimitiveComponent Object Reference") (OtherActor :type "Actor Object Reference") (OtherComp :type "PrimitiveComponent Object Reference") (OtherBodyIndex :type Integer))
  (`SceneComponent.SetVisibility` (`self.Widget`) false false))

(fn `UpdateEnergyBar`
  (`ProgressBar.SetPercent` (`/Game/UI/WB_EnergyBar.EnergyBar` (`self.EnergyBarWB`)) (/ (`self.Energy`) (`self.MaxEnergy`))))

(fn `UserConstructionScript`)