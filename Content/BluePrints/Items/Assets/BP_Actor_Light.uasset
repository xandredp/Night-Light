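; BP_Actor_Light is a switchable point light that also modifies the navmesh around it while lit.
; On BeginPlay it lets every BP_SkinnyMonster affect navigation generation.
; Each Tick it polls IsLightOn to set light visibility and toggle the NavModifier and its sphere, expanding the sphere when on and collapsing it to zero when off.
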(event `self.ReceiveBeginPlay`
  (bind _outactors (`GameplayStatics.GetAllActorsOfClass` "/Game/BluePrints/Enemies/BP_SkinnyMonster.BP_SkinnyMonster_C"))
  (for _array_element _outactors
    (`Pawn.SetCanAffectNavigationGeneration` _array_element true false)))

(event `self.ReceiveTick`
  (params (DeltaSeconds :type "Float (single-precision)"))
  (bind _navmeshmodifiersphere (`self.NavMeshModifierSphere`))
  (bind _navmodifier (`self.NavModifier`))
  (`SceneComponent.SetVisibility` (`self.PointLightComp`) (`self.bIsLightOn`) false)
  (if (`self.bIsLightOn`)
    (`SphereComponent.SetSphereRadius` _navmeshmodifiersphere 150.0 true)
    (`ActorComponent.SetActive` _navmeshmodifiersphere true false)
    (`ActorComponent.SetActive` _navmodifier true false)
    (else
      (`SphereComponent.SetSphereRadius` _navmeshmodifiersphere 0.0 true)
      (`ActorComponent.SetActive` _navmeshmodifiersphere false false)
      (`ActorComponent.SetActive` _navmodifier false false))))

(event `self.ReceiveActorBeginOverlap`
  (params (OtherActor :type "Actor Object Reference")))

(fn `UserConstructionScript`)