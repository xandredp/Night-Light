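; Interactable generator lever switch that outlines when the player is near, unless locked for a specific mechanic.
; Interaction can unlock a linked door and flag listed AI as in light, then rotates the lever behind a one-shot guard.
; Switching on optionally plays a level sequence, blending the view to its camera with player damage disabled, then optionally restores both after a delay.
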(event `self.Lever Highlight Collision Box.OnComponentBeginOverlap`
  (params (OverlappedComponent :type "PrimitiveComponent Object Reference") (OtherActor :type "Actor Object Reference") (OtherComp :type "PrimitiveComponent Object Reference") (OtherBodyIndex :type Integer) (bFromSweep :type Boolean) (SweepResult :type "HitResult Structure (by ref)"))
  ;[1 1 1] Highlighting the mesh with an outline when player gets close
  (if (`self.LockSwitchForSpecificMechanic`)
    ;[1 1 1] Removing the mesh outline highlight
    (cast `/Game/BluePrints/Character/BP_NBCharacter` (stale `self.Lever Highlight Collision Box.OnComponentEndOverlap` OtherActor) :!label _label)
    (`PrimitiveComponent.SetRenderCustomDepth` (`self.PickupMesh`) false)
    (`PrimitiveComponent.SetRenderCustomDepth` (`self.lever`) false)
    (set `self.Action` " ")
    (else
      (cast `/Game/BluePrints/Character/BP_NBCharacter` OtherActor)
      (`PrimitiveComponent.SetRenderCustomDepth` (`self.PickupMesh`) true)
      (`PrimitiveComponent.SetRenderCustomDepth` (`self.lever`) true)
      (set `self.Action` "'E': Turn on generator powered lights"))))

(event `self.Lever Highlight Collision Box.OnComponentEndOverlap`
  (params (OverlappedComponent :type "PrimitiveComponent Object Reference") (OtherActor :type "Actor Object Reference") (OtherComp :type "PrimitiveComponent Object Reference") (OtherBodyIndex :type Integer))
  ;[1 1 1] Removing the mesh outline highlight
  (goto _label))

(event `self.InteractionFeedBack`
  (bind _levercinematic (`self.LeverCinematic`))
  (bind _cameraactor (`self.CameraActor`))
  (bind _lever (`self.lever`))
  (bind _bpdoorleft2 (`self.bpdoorleft2`))
  (bind _aisinlitarea (`self.AIsInLitArea`))
  (bind _lever_2 (`self.lever`))
  (if (not (`self.LockSwitchForSpecificMechanic`))
    (if (`self.IsThereMechanicDoor`)
      ;[1 1 1] begin condition
      (`/Engine/EditorBlueprintResources/StandardMacros.IsValid` _bpdoorleft2
        (:`Is Valid`
          (set `Door.LockDoorForSpecificMechanic` false _bpdoorleft2)
          (if (>= (`KismetArrayLibrary.Array_Length` _aisinlitarea) 0)
            (for _array_element _aisinlitarea
              (bind _output_get (set `NBBaseAI.bisMonsterInLight` true _array_element))
              (`NBBaseAI.MonsterInLight` _array_element _output_get))))))
    (if (not (`self.Interacted`))
      (set `self.Interacted` true)
      (if (`self.IsSwitchOn`)
        (set `self.IsSwitchOn` false)
        (`KismetSystemLibrary.MoveComponentTo` _lever_2 (`SceneComponent.RelativeLocation` _lever_2))
        (else
          (set `self.IsSwitchOn` true)
          (`KismetSystemLibrary.MoveComponentTo` _lever (`SceneComponent.RelativeLocation` _lever) (struct :`Roll` 90.0))
          (if (`self.TolggleSwitch`)
            (`self.ToggleSwitchOnAndOff`))
          ;[1 1 1] Play Anim Seqeunce for lighting
          (`/Engine/EditorBlueprintResources/StandardMacros.IsValid` _levercinematic
            (:`Is Valid`
              (`MovieSceneSequencePlayer.Play` (`LevelSequenceActor.SequencePlayer` _levercinematic))
              (if (`self.SendCameraToSequnce`)
                ;[1 1 1] Set View Target  to   Sequnce Camera
                (`/Engine/EditorBlueprintResources/StandardMacros.IsValid` _cameraactor
                  (:`Is Valid`
                    (`PlayerController.SetViewTargetWithBlend` (`GameplayStatics.GetPlayerController` 0) _cameraactor 0.0 "VTBlend_EaseIn" 0.0 false)
                    ;[1 1 1] Not damage player while playing sequuence
                    (bind _asbp_nbcharacter (cast `/Game/BluePrints/Character/BP_NBCharacter` (`GameplayStatics.GetPlayerCharacter` 0)))
                    (set `NBCharacter.PlayerCanBeDamaged` false _asbp_nbcharacter)
                    (`KismetSystemLibrary.Delay` (`self.lengthofSequence`))
                    (if (`self.ReturnCameraToPlayer`)
                      ;[1 1 1] return camera to player
                      (bind _outactors (`GameplayStatics.GetAllActorsOfClass` "/Game/BluePrints/Character/BP_NBCharacter.BP_NBCharacter_C"))
                      (for (_array_element_2 _array_index) _outactors
                        (bind _asbp_nbcharacter_2 (cast `/Game/BluePrints/Character/BP_NBCharacter` _array_element_2))
                        (set `NBCharacter.PlayerCanBeDamaged` true _asbp_nbcharacter_2)
                        (`PlayerController.SetViewTargetWithBlend` (`GameplayStatics.GetPlayerController` _array_index) _array_element_2 0.0 "VTBlend_Linear" 0.0 false)))))))))))))

(fn `UserConstructionScript`)