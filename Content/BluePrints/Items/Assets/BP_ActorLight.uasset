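; BP_ActorLight is a light actor that switches a spotlight on or off and changes the collision of a linked blocker to match.
; The ToggleSpotLightComp event passes a visibility flag to ToggleLight, which sets SpotLightComp and its children visible or hidden.
; The same flag sets the RELATEDBLOCKER brush's response on the Vehicle channel: Block when lit, Overlap when dark.
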(event `self.ReceiveBeginPlay`)

(event `self.ReceiveActorBeginOverlap`
  (params (OtherActor :type "Actor Object Reference")))

(event `self.ToggleSpotLightComp`
  (params (blightvisiblity :type Boolean))
  (`self.ToggleLight` blightvisiblity))

(fn `ToggleLight`
  (params (blightvisiblity :type Boolean))
  (`SceneComponent.SetVisibility` (`self.SpotLightComp`) blightvisiblity true)
  (if blightvisiblity
    (`PrimitiveComponent.SetCollisionResponseToChannel` (`Brush.BrushComponent` (`self.RELATED BLOCKER`)) "ECC_Vehicle" "ECR_Block")
    (else
      (`PrimitiveComponent.SetCollisionResponseToChannel` (`Brush.BrushComponent` (`self.RELATED BLOCKER`)) "ECC_Vehicle" "ECR_Overlap"))))

(fn `UserConstructionScript`)