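; BP_AmmoPickUp is an ammo box pickup that adds clips to the player's current weapon.
; Its sphere overlap toggles custom depth on the mesh to show an outline highlight while a BP_NBCharacter is in range.
; PickupClips checks the player's current weapon, adds ClipsInBox to its CurrentClip, plays a pickup sound and destroys the actor.
; InteractEvent is an empty stub, and nothing in this graph calls PickupClips.
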(event `self.Sphere.OnComponentBeginOverlap`
  (params (OverlappedComponent :type "PrimitiveComponent Object Reference") (OtherActor :type "Actor Object Reference") (OtherComp :type "PrimitiveComponent Object Reference") (OtherBodyIndex :type Integer) (bFromSweep :type Boolean) (SweepResult :type "HitResult Structure (by ref)"))
  ;[1 1 1] Outline highlight effect
  (cast `/Game/BluePrints/Character/BP_NBCharacter` OtherActor)
  (`PrimitiveComponent.SetRenderCustomDepth` (`self.PickupMesh`) true))

(event `self.Sphere.OnComponentEndOverlap`
  (params (OverlappedComponent :type "PrimitiveComponent Object Reference") (OtherActor :type "Actor Object Reference") (OtherComp :type "PrimitiveComponent Object Reference") (OtherBodyIndex :type Integer))
  ;[1 1 1] Outline highlight effect
  (cast `/Game/BluePrints/Character/BP_NBCharacter` OtherActor)
  (`PrimitiveComponent.SetRenderCustomDepth` (`self.PickupMesh`) false))

(event `self.InteractEvent`)

(event `self.PickupClips`
  (bind _asbp_nbcharacter (cast `/Game/BluePrints/Character/BP_NBCharacter` (`GameplayStatics.GetPlayerCharacter` 0)))
  (bind _currentweapon (`NBCharacter.CurrentWeapon` _asbp_nbcharacter))
  (if (!= _currentweapon null)
    (set `BaseWeapon.CurrentClip` (+ (`BaseWeapon.CurrentClip` _currentweapon) (`self.ClipsInBox`)) _currentweapon)
    (`GameplayStatics.PlaySoundAtLocation` "/Game/Sound/SFX/AmmoPickup/AmmoPickupWav_Cue.AmmoPickupWav_Cue" (`SceneComponent.K2_GetComponentLocation` (`self.PickupMesh`)))
    (`self.K2_DestroyActor`)))

(fn `UserConstructionScript`)