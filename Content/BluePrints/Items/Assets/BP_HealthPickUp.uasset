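; BP_HealthPickUp is an interactable health pickup that heals the player's BP_NBCharacter.
; On InteractEvent it raises player 0's health by IncreaseBy, clamps it to MaxHealth, then destroys itself.
; An OutlineHighlightTrigger toggles custom depth rendering on PickupMesh while a BP_NBCharacter overlaps it, as an outline highlight.
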(event `self.InteractEvent`
  (bind _asbp_nbcharacter (cast `/Game/BluePrints/Character/BP_NBCharacter` (`GameplayStatics.GetPlayerCharacter` 0)))
  (`NBCharacter.IncreaseHealth` _asbp_nbcharacter (`self.IncreaseBy`))
  (bind _maxhealth (`NBCharacter.MaxHealth` _asbp_nbcharacter))
  (if (>= (`NBCharacter.CurrentHealth` _asbp_nbcharacter) _maxhealth)
    (set `NBCharacter.CurrentHealth` _maxhealth _asbp_nbcharacter))
  (`self.K2_DestroyActor`))

(event `self.Outline Highlight Trigger.OnComponentBeginOverlap`
  (params (OverlappedComponent :type "PrimitiveComponent Object Reference") (OtherActor :type "Actor Object Reference") (OtherComp :type "PrimitiveComponent Object Reference") (OtherBodyIndex :type Integer) (bFromSweep :type Boolean) (SweepResult :type "HitResult Structure (by ref)"))
  (cast `/Game/BluePrints/Character/BP_NBCharacter` OtherActor)
  (`PrimitiveComponent.SetRenderCustomDepth` (`self.PickupMesh`) true))

(event `self.Outline Highlight Trigger.OnComponentEndOverlap`
  (params (OverlappedComponent :type "PrimitiveComponent Object Reference") (OtherActor :type "Actor Object Reference") (OtherComp :type "PrimitiveComponent Object Reference") (OtherBodyIndex :type Integer))
  (cast `/Game/BluePrints/Character/BP_NBCharacter` OtherActor)
  (`PrimitiveComponent.SetRenderCustomDepth` (`self.PickupMesh`) false))

(fn `UserConstructionScript`)