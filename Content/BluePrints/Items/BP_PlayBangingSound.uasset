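; An actor that plays a repeating banging sound while the player character is nearby and its linked BPDoor is closed.
; Overlap of BP_NBCharacter with the trigger sphere starts a looping timer that plays the AudioComponent's sound at its location, and leaving clears it.
; Tick polls the door state to gate playback.
; The construction script sizes the sphere from the AudioComponent's attenuation falloff distance.
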(event `self.ReceiveTick`
  (params (DeltaSeconds :type "Float (single-precision)"))
  (if (`Door.IsDoorOpen` (`self.BP_Door`))
    (set `self.bShouldPlaySound` false)
    (else
      (set `self.bShouldPlaySound` true))))

(event `self.Sound Play Trigger.OnComponentBeginOverlap`
  (params (OverlappedComponent :type "PrimitiveComponent Object Reference") (OtherActor :type "Actor Object Reference") (OtherComp :type "PrimitiveComponent Object Reference") (OtherBodyIndex :type Integer) (bFromSweep :type Boolean) (SweepResult :type "HitResult Structure (by ref)"))
  (cast `/Game/BluePrints/Character/BP_NBCharacter` OtherActor)
  (`KismetSystemLibrary.K2_SetTimer` null "Play Sound" 2.0 true))

(event `self.Sound Play Trigger.OnComponentEndOverlap`
  (params (OverlappedComponent :type "PrimitiveComponent Object Reference") (OtherActor :type "Actor Object Reference") (OtherComp :type "PrimitiveComponent Object Reference") (OtherBodyIndex :type Integer))
  (cast `/Game/BluePrints/Character/BP_NBCharacter` OtherActor)
  (`KismetSystemLibrary.K2_ClearTimer` null "Play Sound"))

(fn `Get Attenuation Settings Radius`
  (returns (`Fallof Radius` :type "Float (double-precision)"))
  (locals (Radius :type "Float (double-precision)"))
  (bind _output_get (set `local.Radius` (`.FalloffDistance` (break `SoundAttenuationSettings` (`AudioComponent.AttenuationOverrides` (`self.Audio Component`))))))
  (return _output_get))

(fn `Play Sound`
  (bind _audio_component (`self.Audio Component`))
  (if (`self.bShouldPlaySound`)
    (`GameplayStatics.PlaySoundAtLocation` (`AudioComponent.Sound` _audio_component) (`SceneComponent.K2_GetComponentLocation` _audio_component))))

(fn `UserConstructionScript`
  (bind _fallof_radius (`self.Get Attenuation Settings Radius`))
  (`SphereComponent.SetSphereRadius` (`self.Sound Play Trigger`) _fallof_radius true))