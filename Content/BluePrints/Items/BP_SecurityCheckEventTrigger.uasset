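; A trigger volume that switches on an assigned set of spotlights once the player has fired enough shots while inside it.
; BeginPlay darkens and hides each light in LightsToTurnOn, and BoxTrigger overlaps track whether a BP_NBCharacter is inside.
; While the flag is set, Tick polls the player controller's ShotsFired count against a fixed threshold.
; At the threshold it restores each light's intensity and visibility, repeating every tick without a latch.
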(event `self.Box Trigger.OnComponentBeginOverlap`
  (params (OverlappedComponent :type "PrimitiveComponent Object Reference") (OtherActor :type "Actor Object Reference") (OtherComp :type "PrimitiveComponent Object Reference") (OtherBodyIndex :type Integer) (bFromSweep :type Boolean) (SweepResult :type "HitResult Structure (by ref)"))
  (cast `/Game/BluePrints/Character/BP_NBCharacter` OtherActor)
  (set `self.bPlayerInsideTrigger` true))

(event `self.Box Trigger.OnComponentEndOverlap`
  (params (OverlappedComponent :type "PrimitiveComponent Object Reference") (OtherActor :type "Actor Object Reference") (OtherComp :type "PrimitiveComponent Object Reference") (OtherBodyIndex :type Integer))
  (cast `/Game/BluePrints/Character/BP_NBCharacter` OtherActor)
  (set `self.bPlayerInsideTrigger` false))

(event `self.ReceiveTick`
  (params (DeltaSeconds :type "Float (single-precision)"))
  (if (`self.bPlayerInsideTrigger`)
    (bind _asbp_play_controller (cast `/Game/BluePrints/Core/BP_PlayController` (`Pawn.GetController` (`GameplayStatics.GetPlayerCharacter` 0))))
    (if (>= (`PlayController.ShotsFired` _asbp_play_controller) 6)
      (`self.Trigger Lights To Turn On`))))

(event `self.ReceiveBeginPlay`
  (for _array_element (`self.Lights To Turn On`)
    (bind _spotlight (`/Game/BluePrints/Items/Assets/BP_ActorLight.SpotLight` _array_element))
    (`LightComponent.SetIntensity` _spotlight 0.0)
    (`SceneComponent.SetVisibility` _spotlight false false)))

(event `Trigger Lights To Turn On`
  (for _array_element (`self.Lights To Turn On`)
    (bind _spotlight (`/Game/BluePrints/Items/Assets/BP_ActorLight.SpotLight` _array_element))
    (`LightComponent.SetIntensity` _spotlight (`/Game/BluePrints/Items/Assets/BP_ActorLight.Light Intensity` _array_element))
    (`SceneComponent.SetVisibility` _spotlight true false)))

(fn `UserConstructionScript`)